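; BP_MultiHud is the multiplayer HUD that creates the MultiHudWidget and updates its goal time, player list and game-over display.
; On BeginPlay it binds to the local player state's goal-time dispatcher and the game state's change dispatcher, retrying on short timers until each cast succeeds.
; BindAllPlayerState, not called within this Blueprint, hooks a given player state's goal-time dispatcher and refreshes the list once the widget is valid.
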(event EventBeginPlay
  (bind _returnvalue (UserInterface|CreateWidget "/Game/MultiGame/Widget/MultiHudWidget.MultiHudWidget_C"))
  (bind _output_get (Variables|Default|SetHud _returnvalue))
  (UserInterface|Viewport|AddtoViewport _output_get 0)
  (BindFunc|BindSelfPlayerState)
  (BindFunc|BindGameState))

(fn ConstructionScript)

(fn BindSelfPlayerState
  (bind _asbp_multi_player_state (Utilities|Casting|CastToBP_MultiPlayerState (Variables|/Script/Engine.Controller|GetPlayerState (Game|GetPlayerController 0)))
    (:then
      (EventDispatchers|BindEventtoEventDispatcherUpdateGoalTime _asbp_multi_player_state (EventDispatchers|CreateEvent :!event UpdateGoalTime)))
    (:CastFailed
      (Utilities|Time|SetTimerbyFunctionName 0 "BindSelfPlayerState" 0.1))))

(fn UpdateGoalTime
  (params (GoalTime :type Float%20%28double-precision%29))
  (Default|SetGoalTime (Variables|Default|GetHud) GoalTime))

(fn BindAllPlayerState
  (params (PlayerState :type BP%20Multi%20Player%20State%20Object%20Reference))
  (EventDispatchers|BindEventtoEventDispatcherUpdateGoalTime PlayerState (EventDispatchers|CreateEvent :!event EventUpdateGoalTimes))
  (CallFunction|UpdateAllPlayer))

(fn EventUpdateGoalTimes
  (params (GoalTime :type Float%20%28double-precision%29))
  (Default|UpdatePlayerList (Variables|Default|GetHud)))

(fn UpdateAllPlayer
  (bind _hud (Variables|Default|GetHud))
  (Utilities|IsValid _hud
    (:Is%20Valid
      (Default|UpdatePlayerList _hud))
    (:Is%20Not%20Valid
      (Utilities|Time|SetTimerbyFunctionName 0 "UpdateAllPlayer" 0.1))))

(fn BindGameState
  (bind _asbp_multi_game_state (Utilities|Casting|CastToBP_MultiGameState (Game|GetGameState))
    (:then
      (EventDispatchers|BindEventtoEventDispatcherChangeState _asbp_multi_game_state (EventDispatchers|CreateEvent :!event EventChangeGameState)))
    (:CastFailed
      (Utilities|Time|SetTimerbyFunctionName 0 "BindGameState" 0.1))))

(fn EventChangeGameState
  (params (GameState :type EN_GameState%20Enum :default "NewEnumerator0"))
  (if (Utilities|Enum|Equal(Enum) GameState "NewEnumerator2")
    (Default|DoGameOver (Variables|Default|GetHud))))