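; BP_MultiGameMode is the game mode for a multiplayer game in which characters reach a goal area and have their times recorded.
; Shortly after BeginPlay, a fixed delay elapses and it switches BP_MultiGameState to a new state.
; EnterGoalArea takes the entering character and copies the game state's TotalTime into that character's BP_MultiPlayerState as its goal time.
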(event EventBeginPlay
  (Utilities|FlowControl|Delay 3.0)
  (bind _asbp_multi_game_state (Utilities|Casting|CastToBP_MultiGameState (Game|GetGameState)))
  (Default|ChangeGameState _asbp_multi_game_state "NewEnumerator1"))

(event EventTick
  (params (DeltaSeconds :type Float%20%28single-precision%29)))

(fn ConstructionScript)

(fn EnterGoalArea
  (params (Character :type BP%20Third%20Person%20Character%20Object%20Reference))
  (bind _asbp_multi_player_state (Utilities|Casting|CastToBP_MultiPlayerState (Variables|/Script/Engine.Pawn|GetPlayerState Character)))
  (bind _asbp_multi_game_state (Utilities|Casting|CastToBP_MultiGameState (Game|GetGameState)))
  (Default|SetGoalTime _asbp_multi_player_state (Variables|/Game/MultiGame/GameMode/BP_MultiGameState.BP_MultiGameState_C|GetTotalTime _asbp_multi_game_state)))