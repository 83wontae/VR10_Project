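; BP_MultiPlayerState is the multiplayer player state that records a player's goal time.
; GoalTime uses a RepNotify that fires the UpdateGoalTime event dispatcher whenever the value updates.
; On BeginPlay it passes itself to the first player controller's BP_MultiHud through BindAllPlayerState.
; IsGoalIn treats any goal time above zero as having reached the goal.
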(event EventBeginPlay
  (CallFunction|InitBindCall))

(event EventTick
  (params (DeltaSeconds :type Float%20%28single-precision%29)))

(fn ConstructionScript)

(fn SetGoalTime
  (params (GoalTime :type Float%20%28double-precision%29))
  (Variables|Default|SetGoalTime GoalTime))

(fn OnRepGoalTime
  (Default|CallEventDispatcherUpdateGoalTime (Variables|Default|GetGoalTime)))

(fn InitBindCall
  (bind _asbp_multi_hud (Utilities|Casting|CastToBP_MultiHud (HUD|GetHUD (Game|GetPlayerController 0))))
  (Default|BindAllPlayerState _asbp_multi_hud self))

(fn IsGoalin
  (return (> (Variables|Default|GetGoalTime) 0.0)))