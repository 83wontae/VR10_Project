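; BP_MultiGameState is a multiplayer game state Blueprint that tracks the current game phase and elapsed time.
; Tick adds delta seconds to TotalTime only on the authority.
; ChangeGameState sets the GameState enum and prints its name for debugging.
; GameState uses RepNotify, so OnRep_GameState broadcasts the new value through the ChangeState event dispatcher to any bound listeners.
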(event EventBeginPlay)

(event EventTick
  (params (DeltaSeconds :type Float%20%28single-precision%29))
  (Networking|SwitchHasAuthority
    (:Authority
      (Variables|Default|SetTotalTime (+ (Variables|Default|GetTotalTime) DeltaSeconds)))))

(fn ConstructionScript)

(fn ChangeGameState
  (params (GameState :type EN_GameState%20Enum :default "NewEnumerator0"))
  (bind _output_get (Variables|Default|SetGameState GameState))
  (Development|PrintString (Utilities|String|EnumtoString _output_get)))

(fn OnRepGameState
  (Default|CallEventDispatcherChangeState (Variables|Default|GetGameState)))